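; Player controller that handles the hint overlay, pause menu, game quit and level restart.
; On BeginPlay it shows a WB_Hints widget and hides it after a short delay.
; Escape or P opens a lazily created, reused WB_PauseMenu, switches to UI-only input with a cursor and freezes time through zero global time dilation.
; Events hide the menu and restore play, quit the game, or reopen the FactoryBlockout level.
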(event Custom|OpenPauseMenu
  (bind _pausemenu (Variables|Default|GetPauseMenu)
    (:then
      (Widget|SetVisibility _pausemenu "Visible"))
    (:else
      (bind _returnvalue (UserInterface|CreateWidget "/Game/_Game/UI/WB_PauseMenu.WB_PauseMenu_C"))
      (Variables|Default|SetPauseMenu _returnvalue)
      (UserInterface|Viewport|AddtoViewport (Variables|Default|GetPauseMenu) 0)))
  (Input|SetInputModeUIOnly self (Variables|Default|GetPauseMenu) "LockInFullscreen" false)
  (Variables|Default|SetbShowMouseCursor true)
  (Utilities|Time|SetGlobalTimeDilation 0.0))

(event Custom|HidePauseMenu
  (bind _pausemenu (Variables|Default|GetPauseMenu)
    (:then
      (Widget|SetVisibility _pausemenu "Hidden")
      (Variables|Default|SetbShowMouseCursor false)
      (Input|SetInputModeGameOnly self false)
      (Utilities|Time|SetGlobalTimeDilation 1.0))
    (:else)))

(event Custom|CloseGame
  (Game|QuitGame self "Quit" true))

(event Custom|ReloadGame
  (Game|OpenLevel(byObjectReference) "/Game/Maps/FactoryBlockout.FactoryBlockout")
  (bind _pausemenu (Variables|Default|GetPauseMenu)
    (:then
      (Widget|SetVisibility _pausemenu "Hidden")
      (Variables|Default|SetbShowMouseCursor false)
      (Input|SetInputModeGameOnly self false)
      (Utilities|Time|SetGlobalTimeDilation 1.0))
    (:else)))

(event EventBeginPlay
  (Variables|Default|GetHintMenu
    (:then
      _)
    (:else
      (bind _returnvalue (UserInterface|CreateWidget "/Game/_Game/UI/WB_Hints.WB_Hints_C"))
      (Variables|Default|SetHintMenu _returnvalue)))
  (UserInterface|Viewport|AddtoViewport (Variables|Default|GetHintMenu) 0)
  (Utilities|FlowControl|Delay 5.0)
  (Widget|SetVisibility (Variables|Default|GetHintMenu) "Hidden"))

(event EventTick
  (params (DeltaSeconds :type Float%20%28single-precision%29)))

(event Input|KeyboardEvents|P
  (params (Key :type Key%20Structure :default "None"))
  (:Pressed
    (CallFunction|OpenPauseMenu)))

(event Input|KeyboardEvents|Escape
  (params (Key :type Key%20Structure :default "None"))
  (:Pressed
    (CallFunction|OpenPauseMenu)))

(fn ConstructionScript)